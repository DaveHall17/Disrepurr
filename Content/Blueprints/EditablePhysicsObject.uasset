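; Physics prop with a configurable mesh that can be picked up and dropped, detecting when it stands upright.
; Four trigger boxes recheck their overlaps through a gate that closes on pickup and reopens on drop.
; All four overlapping starts an activation delay that fires Righted and a sound once; fewer cancels it and fires Collapsed.
; FMOD also plays pickup and impact sounds.
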(event `self.Box1.OnComponentBeginOverlap`
  (params (OverlappedComponent :type "PrimitiveComponent Object Reference") (OtherActor :type "Actor Object Reference") (OtherComp :type "PrimitiveComponent Object Reference") (OtherBodyIndex :type Integer) (bFromSweep :type Boolean) (SweepResult :type "HitResult Structure (by ref)"))
  (`/Engine/EditorBlueprintResources/StandardMacros.Gate` false :!label _label
    (:`Exit`
      ;[1 1 1] Check if upright
      (set `self.Int` 0 :!label _label_2)
      (for _array_element (`|MakeArray` (`self.Box1`) (`self.Box2`) (`self.Box3`) (`self.Box4`))
        (`/Engine/EditorBlueprintResources/StandardMacros.CompareInt` (`KismetArrayLibrary.Array_Length` (`PrimitiveComponent.GetOverlappingActors` _array_element null))
          (:`>`
            (`/Engine/EditorBlueprintResources/StandardMacros.IncrementInt` (`self.Int`)))))
      (`/Engine/EditorBlueprintResources/StandardMacros.CompareInt` (`self.Int`) 4
        (:`==`
          (`/Game/Blueprints/DisrepurrMacroLibrary.ACtivationDelay` 1.0 :!label _label_3
            (:`Out`
              (`/Engine/EditorBlueprintResources/StandardMacros.DoOnce` false
                (:`Completed`
                  (`self.Righted`)
                  (`FMODAudioComponent.Play` (`self.FMODAudio`)))))))
        (:`<`
          (`|ExecutionSequence`
            (:`then_0`
              (goto _label_3 :!via `Deactivate`))
            (:`then_1`
              (`self.Collapsed`))))))))

(event `self.Box1.OnComponentEndOverlap`
  (params (OverlappedComponent :type "PrimitiveComponent Object Reference") (OtherActor :type "Actor Object Reference") (OtherComp :type "PrimitiveComponent Object Reference") (OtherBodyIndex :type Integer))
  (goto _label))

(event `self.Box2.OnComponentBeginOverlap`
  (params (OverlappedComponent :type "PrimitiveComponent Object Reference") (OtherActor :type "Actor Object Reference") (OtherComp :type "PrimitiveComponent Object Reference") (OtherBodyIndex :type Integer) (bFromSweep :type Boolean) (SweepResult :type "HitResult Structure (by ref)"))
  (goto _label))

(event `self.Box3.OnComponentBeginOverlap`
  (params (OverlappedComponent :type "PrimitiveComponent Object Reference") (OtherActor :type "Actor Object Reference") (OtherComp :type "PrimitiveComponent Object Reference") (OtherBodyIndex :type Integer) (bFromSweep :type Boolean) (SweepResult :type "HitResult Structure (by ref)"))
  (goto _label))

(event `/Game/Blueprints/PhysicsInterface.Droped`
  (`|ExecutionSequence`
    (:`then_0`
      (goto _label :!via `Open`))
    (:`then_1`
      (goto _label_2))))

(event `self.Box4.OnComponentBeginOverlap`
  (params (OverlappedComponent :type "PrimitiveComponent Object Reference") (OtherActor :type "Actor Object Reference") (OtherComp :type "PrimitiveComponent Object Reference") (OtherBodyIndex :type Integer) (bFromSweep :type Boolean) (SweepResult :type "HitResult Structure (by ref)"))
  (goto _label))

(event `self.Box2.OnComponentEndOverlap`
  (params (OverlappedComponent :type "PrimitiveComponent Object Reference") (OtherActor :type "Actor Object Reference") (OtherComp :type "PrimitiveComponent Object Reference") (OtherBodyIndex :type Integer))
  (goto _label))

(event `/Game/Blueprints/PhysicsInterface.PickedUp`
  (`|ExecutionSequence`
    (:`then_0`
      (goto _label :!via `Close`))
    (:`then_1`
      ;[1 1 1] FMOD
      (`FMODAudioComponent.Play` (`self.FMODAudio_PickUp`)))))

(event `self.Box3.OnComponentEndOverlap`
  (params (OverlappedComponent :type "PrimitiveComponent Object Reference") (OtherActor :type "Actor Object Reference") (OtherComp :type "PrimitiveComponent Object Reference") (OtherBodyIndex :type Integer))
  (goto _label))

(event `self.Box4.OnComponentEndOverlap`
  (params (OverlappedComponent :type "PrimitiveComponent Object Reference") (OtherActor :type "Actor Object Reference") (OtherComp :type "PrimitiveComponent Object Reference") (OtherBodyIndex :type Integer))
  (goto _label))

(event `self.PhysicsMesh.OnComponentHit`
  (params (HitComponent :type "PrimitiveComponent Object Reference") (OtherActor :type "Actor Object Reference") (OtherComp :type "PrimitiveComponent Object Reference") (NormalImpulse :type "Vector Structure") (Hit :type "HitResult Structure (by ref)"))
  ;[1 1 1] FMOD
  (`/Game/Blueprints/DisrepurrMacroLibrary.FMOD_HitSounds` 0.2 1000.0 Hit (`self.FMODAudio_Hit`) NormalImpulse))

(fn `GetPhysicsComponent`
  (returns (PhysicsMesh :type "PrimitiveComponent Object Reference"))
  (bind _physicsmesh (`self.PhysicsMesh`))
  (return (select `bool` (`SceneComponent.IsSimulatingPhysics` _physicsmesh "None") :`true` _physicsmesh)))

(fn `UserConstructionScript`
  (`StaticMeshComponent.SetStaticMesh` (`self.PhysicsMesh`) (`self.StaticMesh`)))