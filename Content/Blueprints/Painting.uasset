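; Painting Blueprint for a placeable painting prop whose mesh can be switched between static and physics-simulated.
; The construction script applies the chosen static mesh and sets its initial simulation state from StartAwake.
; A SetPhysics event toggles simulation at runtime.
; GetPhysicsComponent exposes the mesh to callers only while it is simulating physics.
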(event `SetPhysics`
  (params (`Simulate?` :type Boolean :default true))
  (`PrimitiveComponent.SetSimulatePhysics` (`self.PaintingMesh`) `Simulate?`))

(fn `GetPhysicsComponent`
  (returns (PhysicsMesh :type "PrimitiveComponent Object Reference"))
  (bind _paintingmesh (`self.PaintingMesh`))
  (return (select `bool` (`SceneComponent.IsSimulatingPhysics` _paintingmesh "None") :`true` _paintingmesh :!type "PrimitiveComponent Object Reference")))

(fn `UserConstructionScript`
  (bind _paintingmesh (`self.PaintingMesh`))
  (`PrimitiveComponent.SetSimulatePhysics` _paintingmesh (`self.StartAwake?`))
  (`StaticMeshComponent.SetStaticMesh` _paintingmesh (`self.StaticMesh`)))