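; A target zone for a specific painting that snaps it into place, with its area mesh and overlap box sized in the construction script.
; Box overlaps enable Tick while the target painting is inside, checking its location and rotation against target values within tolerances.
; A match feeds a retriggerable delay and gate into PaintingInPosition, which stops Tick, disables physics and uses a timeline to lerp the painting's transform to the target.
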(event `self.Box.OnComponentBeginOverlap`
  (params (OverlappedComponent :type "PrimitiveComponent Object Reference") (OtherActor :type "Actor Object Reference") (OtherComp :type "PrimitiveComponent Object Reference") (OtherBodyIndex :type Integer) (bFromSweep :type Boolean) (SweepResult :type "HitResult Structure (by ref)"))
  (if (`KismetArrayLibrary.Array_Contains` (`PrimitiveComponent.GetOverlappingActors` (`self.Box`) "/Game/Blueprints/Painting.Painting_C") (`self.TargetPainting`)) :!label _label
    (`KismetSystemLibrary.PrintString` "Overlapping")
    (`self.SetActorTickEnabled` true)
    (else
      (`KismetSystemLibrary.PrintString` "Not Overalpin")
      (`self.SetActorTickEnabled` false))))

(event `self.Box.OnComponentEndOverlap`
  (params (OverlappedComponent :type "PrimitiveComponent Object Reference") (OtherActor :type "Actor Object Reference") (OtherComp :type "PrimitiveComponent Object Reference") (OtherBodyIndex :type Integer))
  (goto _label))

(event `self.ReceiveTick`
  (params (DeltaSeconds :type "Float (single-precision)"))
  (`KismetSystemLibrary.PrintString` "Check Postion")
  (if (== (`self.K2_GetActorLocation` (`self.TargetPainting`)) (`self.targetLocation`) :`ErrorTolerance` 25.0)
    (if (== (`self.K2_GetActorRotation` (`self.TargetPainting`)) (`self.TargetRotation`) :`ErrorTolerance` 10.0)
      (`KismetSystemLibrary.PrintString` "In correct postion")
      (`|ExecutionSequence`
        (:`then_0`
          (`KismetSystemLibrary.RetriggerableDelay` 0.5)
          (`/Engine/EditorBlueprintResources/StandardMacros.Gate` true :!label _label_2
            (:`Exit`
              (`self.PaintingInPosition`))))
        (:`then_1`
          (goto _label_2 :!via `Open`)))
      (else
        (`KismetSystemLibrary.PrintString` "Rotation Wornd")
        (goto _label_2 :!via `Close`)))
    (else
      (`KismetSystemLibrary.PrintString` "Postion Worngf")
      (goto _label_2 :!via `Close`))))

(event `PaintingInPosition`
  (bind _physicsmesh (`self.PhysicsMesh`))
  (`self.SetActorTickEnabled` false)
  (bind _targetpainting (`self.TargetPainting`)
    (:`then`
      (bind _output_get (set `self.PhysicsMesh` (`/Game/Blueprints/Painting.Base` _targetpainting)))
      (`PrimitiveComponent.SetSimulatePhysics` _output_get false)
      (set `self.StartPosition` (`SceneComponent.K2_GetComponentLocation` _physicsmesh))
      (set `self.StartRotation` (`SceneComponent.K2_GetComponentRotation` _physicsmesh))
      (bind (_direction _lerp) (`Timeline|SnapTimeline` :!via `PlayFromStart`)
        (:`Update`
          (`SceneComponent.K2_SetWorldTransform` (`self.PhysicsMesh`) (`KismetMathLibrary.MakeTransform` (`KismetMathLibrary.VLerp` (`self.StartPosition`) (`self.targetLocation`) _lerp) (`KismetMathLibrary.RLerp` (`self.StartRotation`) (`self.TargetRotation`) _lerp true) (`KismetMathLibrary.VLerp` (1.0 1.0 1.0) (1.0 1.1 1.0) _lerp)) false false))))
    (:`else`)))

(fn `UserConstructionScript`
  (bind (_paintingscale_x _paintingscale_y) (`KismetMathLibrary.BreakVector2D` (`self.PaintingScale`)))
  (`SceneComponent.K2_SetRelativeTransform` (`self.AreaMesh`) (`KismetMathLibrary.MakeTransform` (`KismetMathLibrary.MakeVector` (`self.PaintingOffset_Float`) 0.0 0.1) (struct) (`KismetMathLibrary.MakeVector` _paintingscale_x _paintingscale_y 1.0)) false false)
  (`SceneComponent.K2_SetRelativeTransform` (`self.Box`) (`KismetMathLibrary.MakeTransform` (`KismetMathLibrary.MakeVector` (`self.PaintingOffset_Float`) 0.0 0.1) (struct) (`KismetMathLibrary.MakeVector` _paintingscale_x _paintingscale_y 1.0)) false false))