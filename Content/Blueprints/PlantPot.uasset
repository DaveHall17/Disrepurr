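; Physics plant pot that detects being stood upright and broadcasts a one-time righted event.
; Begin and end overlaps on the base trigger activate a delay component while anything overlaps and deactivate it when empty; its output fires the dispatcher and a fixed sound once.
; Pickup and hit events play FMOD audio, with hits passing their impulse along.
; The construction script applies the configurable mesh, which serves as the physics component while simulating.
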(event `self.PotBaseTrigger.OnComponentBeginOverlap`
  (params (OverlappedComponent :type "PrimitiveComponent Object Reference") (OtherActor :type "Actor Object Reference") (OtherComp :type "PrimitiveComponent Object Reference") (OtherBodyIndex :type Integer) (bFromSweep :type Boolean) (SweepResult :type "HitResult Structure (by ref)"))
  (`/Engine/EditorBlueprintResources/StandardMacros.CompareInt` (`KismetArrayLibrary.Array_Length` (`PrimitiveComponent.GetOverlappingActors` (`self.PotBaseTrigger`) null)) :!label _label
    (:`>`
      (`/Game/Blueprints/DisrepurrMacroLibrary.ACtivationDelay` 1.0 :!label _label_2
        (:`Out`
          (`/Engine/EditorBlueprintResources/StandardMacros.DoOnce` false
            (:`Completed`
              (`self.PlatPotRighted`)
              (`KismetSystemLibrary.PrintString` "Stand Up")
              (`FMODAudioComponent.Play` (`self.FMODAudio_Fixed`)))))))
    (:`==`
      (goto _label_2 :!via `Deactivate`))))

(event `self.PotBaseTrigger.OnComponentEndOverlap`
  (params (OverlappedComponent :type "PrimitiveComponent Object Reference") (OtherActor :type "Actor Object Reference") (OtherComp :type "PrimitiveComponent Object Reference") (OtherBodyIndex :type Integer))
  (goto _label))

(event `/Game/Blueprints/PhysicsInterface.PickedUp`
  ;[1 1 1] FMOD
  (`FMODAudioComponent.Play` (`self.FMODAudio_PickUp`)))

(event `self.PlantPot.OnComponentHit`
  (params (HitComponent :type "PrimitiveComponent Object Reference") (OtherActor :type "Actor Object Reference") (OtherComp :type "PrimitiveComponent Object Reference") (NormalImpulse :type "Vector Structure") (Hit :type "HitResult Structure (by ref)"))
  ;[1 1 1] FMOD
  (`/Game/Blueprints/DisrepurrMacroLibrary.FMOD_HitSounds` 0.2 1000.0 Hit (`self.FMODAudio_Hit`) NormalImpulse))

(fn `GetPhysicsComponent`
  (returns (PhysicsMesh :type "PrimitiveComponent Object Reference"))
  (bind _plantpot (`self.PlantPot`))
  (return (select `bool` (`SceneComponent.IsSimulatingPhysics` _plantpot "None") :`true` _plantpot)))

(fn `UserConstructionScript`
  (`StaticMeshComponent.SetStaticMesh` (`self.PlantPot`) (`self.PlantPotMesh`)))