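; Lamp is a physics prop that accepts a LightBulb in its socket and lights it.
; When the bulb's attachment point overlaps LampAttachmentPoint, gates and a short retriggerable delay lead to AttachLightBulb, which also runs on BeginPlay for a preset bulb.
; It disables bulb physics, timeline-lerps it into place, turns it on, attaches it to Base and calls CallLampTurnedOn.
; The construction script sets mesh and socket position; FMOD handles pickup and impact sounds.
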(event `self.LampAttachmentPoint.OnComponentBeginOverlap`
  (params (OverlappedComponent :type "PrimitiveComponent Object Reference") (OtherActor :type "Actor Object Reference") (OtherComp :type "PrimitiveComponent Object Reference") (OtherBodyIndex :type Integer) (bFromSweep :type Boolean) (SweepResult :type "HitResult Structure (by ref)"))
  ;[1 1 1] Overlaps
  (`/Engine/EditorBlueprintResources/StandardMacros.Gate` false :!label _label
    (:`Exit`
      (bind _aslight_bulb (cast `/Game/Blueprints/LightBulb` (`|GetArrayItem` (`self.GetOverlappingActors` "/Game/Blueprints/LightBulb.LightBulb_C")))
        (:`then`
          (set `self.LightBulb` _aslight_bulb)
          (if (`PrimitiveComponent.IsOverlappingComponent` (`/Game/Blueprints/LightBulb.BulbAttachmentPoint` _aslight_bulb) (`self.LampAttachmentPoint`))
            (`KismetSystemLibrary.PrintString` "Hello")
            (`|ExecutionSequence`
              (:`then_0`
                (`KismetSystemLibrary.RetriggerableDelay` 0.25)
                (`/Engine/EditorBlueprintResources/StandardMacros.Gate` true :!label _label_2
                  (:`Exit`
                    (`self.AttachLightBulb`))))
              (:`then_1`
                (goto _label_2 :!via `Open`)))
            (else
              (`KismetSystemLibrary.PrintString` "Bye" :!label _label_3)
              (goto _label_2 :!via `Close`))))
        (:`CastFailed`
          (goto _label_3))))))

(event `self.LampAttachmentPoint.OnComponentEndOverlap`
  (params (OverlappedComponent :type "PrimitiveComponent Object Reference") (OtherActor :type "Actor Object Reference") (OtherComp :type "PrimitiveComponent Object Reference") (OtherBodyIndex :type Integer))
  ;[1 1 1] Overlaps
  (goto _label))

(event `AttachLightBulb`
  (bind _lampattachmentpoint (`self.LampAttachmentPoint`))
  ;[1 1 1] Light bulb in place
  (bind _lightbulb (`self.LightBulb` :!label _label_4)
    (:`then`
      (bind _physicsmesh (message `/Game/Blueprints/PhysicsInterface.GetPhysicsComponent` _lightbulb))
      (set `self.PhysicsMesh` _physicsmesh)
      (`PrimitiveComponent.SetSimulatePhysics` (`self.PhysicsMesh`) false)
      (`|ExecutionSequence`
        (:`then_0`
          (goto _label :!via `Close`))
        (:`then_1`
          (set `self.StartPosition` (`SceneComponent.K2_GetComponentLocation` (`self.PhysicsMesh`)))
          (set `self.StartRotation` (`SceneComponent.K2_GetComponentRotation` (`self.PhysicsMesh`)))
          (bind (_direction _lerp) (`Timeline|SNapTimeline` :!via `PlayFromStart`)
            (:`Update`
              (`SceneComponent.K2_SetWorldLocationAndRotation` (`self.PhysicsMesh`) (`KismetMathLibrary.VLerp` (`self.StartPosition`) (`SceneComponent.K2_GetComponentLocation` _lampattachmentpoint) _lerp) (`KismetMathLibrary.RLerp` (`self.StartRotation`) (`SceneComponent.K2_GetComponentRotation` _lampattachmentpoint) _lerp true) false false))
            (:`Finished`
              (`/Game/Blueprints/LightBulb.TurnLightOn` (`self.LightBulb`))
              (`SceneComponent.K2_AttachToComponent` (`self.PhysicsMesh`) (`self.Base`) "None" "KeepWorld" "KeepWorld" "KeepWorld" true)
              (`self.LampTurnedOn`))))))
    (:`else`)))

(event `self.ReceiveBeginPlay`
  ;[1 1 1] Light bulb in place
  (goto _label_4))

(event `/Game/Blueprints/PhysicsInterface.PickedUp`
  ;[1 1 1] FMOD
  (`FMODAudioComponent.Play` (`self.FMODAudio_PickUp`)))

(event `self.Base.OnComponentHit`
  (params (HitComponent :type "PrimitiveComponent Object Reference") (OtherActor :type "Actor Object Reference") (OtherComp :type "PrimitiveComponent Object Reference") (NormalImpulse :type "Vector Structure") (Hit :type "HitResult Structure (by ref)"))
  ;[1 1 1] FMOD
  (`/Game/Blueprints/DisrepurrMacroLibrary.FMOD_HitSounds` 0.2 1000.0 Hit (`self.FMODAudio_Hit`) NormalImpulse))

(fn `GetPhysicsComponent`
  (returns (PhysicsMesh :type "PrimitiveComponent Object Reference"))
  (return (`self.Base`)))

(fn `UserConstructionScript`
  (`StaticMeshComponent.SetStaticMesh` (`self.Base`) (`self.LampMesh`))
  (`SceneComponent.K2_SetRelativeLocation` (`self.LampAttachmentPoint`) (`self.LightPosition`) false false))