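; FixedPipe is a fixed fitting that snaps loose Pipe actors into place.
; Begin and end overlaps on its two spheres check each overlapping Pipe; one not touching both triggers AttachPipe, while full contact only prints.
; AttachPipe disables physics and runs a timeline transform on the pipe mesh.
; Start values come from the target component itself, so position and rotation jump there immediately while only Y scale visibly stretches.
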(event `self.Sphere2.OnComponentBeginOverlap`
  (params (OverlappedComponent :type "PrimitiveComponent Object Reference") (OtherActor :type "Actor Object Reference") (OtherComp :type "PrimitiveComponent Object Reference") (OtherBodyIndex :type Integer) (bFromSweep :type Boolean) (SweepResult :type "HitResult Structure (by ref)"))
  ;[1 1 1] Check Overlaps
  (for _array_element (`self.GetOverlappingActors` "/Game/Blueprints/Pipe.Pipe_C") :!label _label
    (bind _aspipe (cast `/Game/Blueprints/Pipe` _array_element))
    (set `self.OverlappingPipe` _aspipe)
    (if (`PrimitiveComponent.IsOverlappingActor` (`self.Sphere1`) (`self.OverlappingPipe`))
      (if (`PrimitiveComponent.IsOverlappingActor` (`self.Sphere2`) (`self.OverlappingPipe`))
        (`KismetSystemLibrary.PrintString` "Attached at both ends")
        (else
          (`KismetSystemLibrary.PrintString` "Not Attached properly" :!label _label_2)
          (`self.AttachPipe`)))
      (else
        (goto _label_2)))))

(event `self.Sphere1.OnComponentBeginOverlap`
  (params (OverlappedComponent :type "PrimitiveComponent Object Reference") (OtherActor :type "Actor Object Reference") (OtherComp :type "PrimitiveComponent Object Reference") (OtherBodyIndex :type Integer) (bFromSweep :type Boolean) (SweepResult :type "HitResult Structure (by ref)"))
  ;[1 1 1] Check Overlaps
  (goto _label))

(event `self.Sphere2.OnComponentEndOverlap`
  (params (OverlappedComponent :type "PrimitiveComponent Object Reference") (OtherActor :type "Actor Object Reference") (OtherComp :type "PrimitiveComponent Object Reference") (OtherBodyIndex :type Integer))
  ;[1 1 1] Check Overlaps
  (goto _label))

(event `self.Sphere1.OnComponentEndOverlap`
  (params (OverlappedComponent :type "PrimitiveComponent Object Reference") (OtherActor :type "Actor Object Reference") (OtherComp :type "PrimitiveComponent Object Reference") (OtherBodyIndex :type Integer))
  ;[1 1 1] Check Overlaps
  (goto _label))

(event `AttachPipe`
  (bind _targetpostion (`self.TargetPostion`))
  (bind _returnvalue (`SceneComponent.K2_GetComponentLocation` _targetpostion))
  (bind _returnvalue_2 (`SceneComponent.K2_GetComponentRotation` _targetpostion))
  (bind _overlappingpipe (`self.OverlappingPipe`)
    (:`then`
      (`PrimitiveComponent.SetSimulatePhysics` (`/Game/Blueprints/Pipe.PhysicsMesh` _overlappingpipe) false)
      (set `self.StartPosition` _returnvalue)
      (set `self.StartRotation` _returnvalue_2)
      (bind (_direction _lerp) (`Timeline|SnapIntoPlace` :!via `PlayFromStart`)
        (:`Update`
          (`SceneComponent.K2_SetWorldTransform` (`/Game/Blueprints/Pipe.PhysicsMesh` (`self.OverlappingPipe`)) (`KismetMathLibrary.MakeTransform` (`KismetMathLibrary.VLerp` (`self.StartPosition`) _returnvalue _lerp) (`KismetMathLibrary.RLerp` (`self.StartRotation`) _returnvalue_2 _lerp true) (`KismetMathLibrary.VLerp` (1.0 1.0 1.0) (1.0 1.1 1.0) _lerp)) false false))))
    (:`else`)))

(fn `UserConstructionScript`)