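; Light bulb Blueprint that can be switched on, with a Bulb component and a point light.
; The construction script creates a dynamic material instance from LightMaterial, stores it back in that variable and applies it to the Bulb.
; TurnLightOn gives that material an overbright warm colour, sets its opacity and raises the point light's intensity, with no matching off event.
; GetPhysicsComponent returns the Bulb when it is simulating physics.
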(event `TurnLightOn`
  (bind _lightmaterial (`self.LightMaterial`))
  (`MaterialInstanceDynamic.SetVectorParameterValue` _lightmaterial "LightColour" (struct :`R` 10.0 :`G` 10.0 :`B` 5.0 :`A` 1.0))
  (`MaterialInstanceDynamic.SetScalarParameterValue` _lightmaterial "Opacity" 0.8)
  (`LightComponent.SetIntensity` (`self.PointLight`) 10000.0))

(fn `GetPhysicsComponent`
  (returns (PhysicsMesh :type "PrimitiveComponent Object Reference"))
  (bind _bulb (`self.Bulb`))
  (return (select `bool` (`SceneComponent.IsSimulatingPhysics` _bulb "None") :`true` _bulb)))

(fn `UserConstructionScript`
  (bind _returnvalue (`KismetMaterialLibrary.CreateDynamicMaterialInstance` "/Game/Blueprints/Materials/LightMaterial.LightMaterial"))
  (bind _output_get (set `self.LightMaterial` _returnvalue))
  (`PrimitiveComponent.SetMaterial` (`self.Bulb`) 0 _output_get))