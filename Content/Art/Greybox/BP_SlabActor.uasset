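; BP_SlabActor is a greybox building block that becomes a box mesh, a cylinder mesh or an invisible collision box with an icon.
; Its construction script applies the slab type, then sizes and centers the mesh and collision box from paired X, Y and Z points.
; It then moves the actor pivot to the slab center and re-offsets each point, constraining it to its own axis.
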(fn `ConstrainSlabMovement`
  ;[0.06688 0.07 0.0263] Constrainers WITH PIVOT OFFSET
  (set `self.Z+` (`KismetMathLibrary.MakeVector` (`self.X Center`) (`self.Y Center`) (.z (- (`self.Z+`) (`self.Point Offset`)))))
  (set `self.Z-` (`KismetMathLibrary.MakeVector` (`self.X Center`) (`self.Y Center`) (.z (- (`self.Z-`) (`self.Point Offset`)))))
  (set `self.X+` (`KismetMathLibrary.MakeVector` (.x (- (`self.X+`) (`self.Point Offset`))) (`self.Y Center`) (`self.Z Center`)))
  (set `self.X-` (`KismetMathLibrary.MakeVector` (.x (- (`self.X-`) (`self.Point Offset`))) (`self.Y Center`) (`self.Z Center`)))
  (set `self.Y+` (`KismetMathLibrary.MakeVector` (`self.X Center`) (.y (- (`self.Y+`) (`self.Point Offset`))) (`self.Z Center`)))
  (set `self.Y-` (`KismetMathLibrary.MakeVector` (`self.X Center`) (.y (- (`self.Y-`) (`self.Point Offset`))) (`self.Z Center`))))

(fn `SetPivotPosition`
  (bind _returnvalue (`SceneComponent.K2_GetComponentLocation` (`self.SlabMesh`)))
  ;[1 0.255 0.6426] Get pivot offset and set root position
  (`self.K2_SetActorLocation` _returnvalue)
  (set `self.Point Offset` (`KismetMathLibrary.InverseTransformLocation` (`self.GetTransform`) _returnvalue)))

(fn `SetSlabScale`
  (bind _returnvalue (/ (+ (`self.X+`) (`self.X-`)) 2))
  (bind _returnvalue_2 (/ (+ (`self.Z+`) (`self.Z-`)) 2))
  (bind _returnvalue_3 (/ (+ (`self.Y+`) (`self.Y-`)) 2))
  (bind _returnvalue_4 (`KismetMathLibrary.MakeVector` (.x _returnvalue) (.y _returnvalue_3) (.z _returnvalue_2)))
  (bind _returnvalue_5 (/ (`KismetMathLibrary.MakeVector` (* (`KismetMathLibrary.VSize` (- (`self.X-`) _returnvalue)) 2.0) (* (`KismetMathLibrary.VSize` (- (`self.Y-`) _returnvalue_3)) 2.0) (* (`KismetMathLibrary.VSize` (- (`self.Z-`) _returnvalue_2)) 2.0)) 100.0))
  ;[1 1 0.146] Set Centers of Axis for constraints
  (set `self.X Center` (.x _returnvalue))
  (set `self.Y Center` (.y _returnvalue_3))
  (set `self.Z Center` (.z _returnvalue_2))
  ;[1 1 0.146] Make Slab Location, set slab relative location and relative scale
  (`SceneComponent.K2_SetRelativeLocation` (`self.SlabMesh`) _returnvalue_4 false false)
  (`SceneComponent.SetRelativeScale3D` (`self.SlabMesh`) _returnvalue_5)
  (`SceneComponent.K2_SetRelativeLocation` (`self.SlabBox`) _returnvalue_4 false false)
  (`SceneComponent.SetRelativeScale3D` (`self.SlabBox`) _returnvalue_5)
  (return))

(fn `SetupSlabType`
  (bind _slabbox (`self.SlabBox`))
  (bind _icon (`self.ICON`))
  (bind _slabmesh (`self.SlabMesh`))
  ;[1 1 1] Switch Type of Slab
  (`StaticMeshComponent.SetStaticMesh` (`self.SlabMesh`) (`self.StaticMesh`))
  (switch `/LevelSlabs/Enum_SlabType` (`self.SlabType`)
    (:`NewEnumerator0`
      (`StaticMeshComponent.SetStaticMesh` _slabmesh "/Engine/BasicShapes/Cube.Cube")
      (`PrimitiveComponent.SetCollisionEnabled` _slabbox "NoCollision" :!label _label)
      (`SceneComponent.SetVisibility` _icon false true))
    (:`NewEnumerator1`
      (`StaticMeshComponent.SetStaticMesh` _slabmesh "/Engine/BasicShapes/Cylinder.Cylinder")
      (goto _label))
    (:`NewEnumerator2`
      (`StaticMeshComponent.SetStaticMesh` _slabmesh null)
      (`PrimitiveComponent.SetCollisionEnabled` _slabbox "QueryAndPhysics")
      (`SceneComponent.SetVisibility` _icon true true)))
  (return))

(fn `UserConstructionScript`
  (locals (`Bounds Center` :type "Vector Structure" :default (0.0 0.0 0.0)) (`Bounds Extent` :type "Vector Structure" :default (0.0 0.0 0.0)) (`Original Location` :type "Vector Structure" :default (0.0 0.0 0.0)))
  ;[1 1 1] Slab Construction Script
  (`self.SetupSlabType`)
  (`self.SetSlabScale`)
  (`self.SetPivotPosition`)
  (`self.ConstrainSlabMovement`))